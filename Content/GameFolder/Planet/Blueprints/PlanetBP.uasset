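; Planet actor that spins the planet, moon and thunder, and creates and drives the main HUD.
; Menu buttons move the player pawn along X/Y timelines and handle input mode and pausing.
; Tick polls HUD state: full Technology triggers a delayed rocket launch revealing a satellite, and overheating drives a fire atmosphere through a material parameter collection.
; A box overlap randomly enables moon shadow casting for a while.
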(event OnComponentBeginOverlap(Box)
  (params (OverlappedComponent :type Primitive%20Component%20Object%20Reference) (OtherActor :type Actor%20Object%20Reference) (OtherComp :type Primitive%20Component%20Object%20Reference) (OtherBodyIndex :type Integer) (bFromSweep :type Boolean) (SweepResult :type Hit%20Result%20Structure%20%28by%20ref%29))
  (bind _moon (Variables|Default|GetMoon))
  (if (Collision|IsOverlappingActor (Variables|Default|GetMoon) OtherActor :!class /Script/Engine.PrimitiveComponent)
    (switch int (Math|Random|RandomInteger 9)
      (:Default
        (Rendering|SetCastShadow _moon true :!label _label)
        (Utilities|FlowControl|Delay 45.0)
        (Rendering|SetCastShadow _moon false))
      (:0
        (goto _label))
      (:1
        (Rendering|SetCastShadow _moon false))
      (:2
        (Rendering|SetCastShadow _moon false))
      (:3
        (Rendering|SetCastShadow _moon false))
      (:4
        (Rendering|SetCastShadow _moon false))
      (:5
        (Rendering|SetCastShadow _moon false))
      (:6
        (Rendering|SetCastShadow _moon false))
      (:7
        (Rendering|SetCastShadow _moon false))
      (:8
        (Rendering|SetCastShadow _moon false))
      (:9
        (Rendering|SetCastShadow _moon false)))))

(event Custom|MenuButtonClicked
  (bind _main_hud (Variables|Default|GetMain%20HUD))
  (bind _main_hud_2 (Variables|Default|GetMain%20HUD))
  (bind _fade_hud (Variables|/Game/GameFolder/Player/PlayerHUD/Main_HUD.Main_HUD_C|GetFade%20HUD _main_hud))
  ;[1 1 1] Menu Button
  (Utilities|FlowControl|Sequence
    (:then_0
      (Transformation|SetWorldRotation (Variables|/Game/GameFolder/Player/Player_Pawn.Player_Pawn_C|GetSpringArm (Utilities|Array|Get(acopy) (stale EventTick _outactors))) "0,-90.000000, 0" false false)
      (Input|SetInputModeUIOnly (Game|GetPlayerController 0) 0 "DoNotLock")
      (Utilities|FlowControl|Sequence
        (:then_0
          (bind _x (Timeline|X Play)
            (:Update
              (Transformation|SetWorldLocationAndRotation (Variables|/Game/GameFolder/Player/Player_Pawn.Player_Pawn_C|GetDefaultSceneRoot (Utilities|Array|Get(acopy) (stale EventTick _outactors))) (Math|Vector|MakeVector _x (stale _y) 0.0) "0,-90.000000, 0" false false :!label _label))
            (:Finished
              (Utilities|FlowControl|FlipFlop
                (:A
                  (Utilities|FlowControl|Delay 0.05)
                  (Game|SetGamePaused true))))))
        (:then_1
          (bind _y (Timeline|Y Play)
            (:Update
              (goto _label))))))
    (:then_1
      (Utilities|FlowControl|DoOnce false
        (:Completed
          (UserInterface|Animation|PlayAnimation _main_hud _fade_hud 0.0 1 "Forward" 1.0)
          (Utilities|FlowControl|Delay 1.5)
          (Class|UserWidget|PauseAnimation _main_hud _fade_hud))))
    (:then_2
      (Utilities|FlowControl|DoOnce false) ; enters at Reset
    )))

(event Custom|BackButtonClicked
  (bind _main_hud (Variables|Default|GetMain%20HUD))
  (bind _main_hud_2 (Variables|Default|GetMain%20HUD))
  (bind _fade_hud (Variables|/Game/GameFolder/Player/PlayerHUD/Main_HUD.Main_HUD_C|GetFade%20HUD _main_hud))
  ;[1 1 1] Menu Button
  (if (Game|IsGamePaused)
    (Utilities|FlowControl|Sequence
      (:then_0
        (Game|SetGamePaused false)
        (Input|SetInputModeGameandUI (Game|GetPlayerController 0) 0 "DoNotLock" true)
        (Utilities|FlowControl|Sequence
          (:then_0
            (bind _x (Timeline|X Reverse)
              (:Update
                (Transformation|SetWorldLocationAndRotation (Variables|/Game/GameFolder/Player/Player_Pawn.Player_Pawn_C|GetDefaultSceneRoot (Utilities|Array|Get(acopy) (stale EventTick _outactors))) (Math|Vector|MakeVector _x (stale _y) 0.0) "0,-90.000000, 0" false false :!label _label))
              (:Finished
                (Utilities|FlowControl|FlipFlop
                  (:A
                    (Utilities|FlowControl|Delay 0.05)
                    (Game|SetGamePaused true))))))
          (:then_1
            (bind _y (Timeline|Y Reverse)
              (:Update
                (goto _label))))))
      (:then_1
        (Utilities|FlowControl|DoOnce false) ; enters at Reset
      )
      (:then_2
        (Utilities|FlowControl|DoOnce false
          (:Completed
            (Utilities|FlowControl|Delay 3.0)
            (UserInterface|Animation|PlayAnimation _main_hud_2 (Variables|/Game/GameFolder/Player/PlayerHUD/Main_HUD.Main_HUD_C|GetFade%20HUD _main_hud_2) 0.0 1 "Reverse" 1.0)))))))

(event EventBeginPlay
  ;[1 1 1] Set Main HUD
  (Utilities|FlowControl|Sequence
    (:then_0
      (bind _returnvalue (UserInterface|CreateWidget "/Game/GameFolder/Player/PlayerHUD/Main_HUD.Main_HUD_C"))
      (UserInterface|Viewport|AddtoViewport _returnvalue 0)
      (Input|SetInputModeGameandUI (Game|GetPlayerController 0) _returnvalue "DoNotLock" true))))

(event EventTick
  (params (DeltaSeconds :type Float%20%28single-precision%29))
  (bind _rotationspeed (Variables|Default|GetRotationSpeed))
  (bind _rocket (Variables|Default|GetRocket))
  (bind _returnvalue (* DeltaSeconds _rotationspeed))
  ;[1 1 1] Planet and weather rotation
  (Utilities|FlowControl|Sequence
    (:then_0
      (Transformation|AddLocalRotation (Variables|Debug|GetStaticMeshComponent) (Math|Rotator|MakeRotator 0.0 0.0 _returnvalue) false false))
    (:then_1
      (Transformation|AddLocalRotation (Variables|Default|GetMoon) (Math|Rotator|MakeRotator 0.0 0.0 _returnvalue) false false))
    (:then_2
      (Transformation|AddLocalRotation (Variables|Default|GetSpringArm) (Math|Rotator|MakeRotator 0.0 0.0 1e-18) false false))
    (:then_3
      (Transformation|AddLocalRotation (Variables|Default|GetThunder) (Math|Rotator|MakeRotator 0.0 0.0 0.0005) false false))
    (:then_4
      ;[1 1 1] Menu Button
      (Utilities|FlowControl|Sequence
        (:then_0
          (Utilities|FlowControl|Sequence
            (:then_0
              (if (<= (stale _output_get) -1.01e+03)
                (Appearance|SetColorandOpacity (Variables|/Game/GameFolder/Player/PlayerHUD/Main_HUD.Main_HUD_C|GetMenu_HUD_359 (Variables|Default|GetMain%20HUD)) "(R=1.000000,G=1.000000,B=1.000000,A=1.000000)" :!class /Script/UMG.UserWidget)
                (else
                  (Appearance|SetColorandOpacity (Variables|/Game/GameFolder/Player/PlayerHUD/Main_HUD.Main_HUD_C|GetMenu_HUD_359 (Variables|Default|GetMain%20HUD)) "(R=1.000000,G=1.000000,B=1.000000,A=0.000000)" :!class /Script/UMG.UserWidget))))
            (:then_1
              (bind _output_get (Variables|Default|SetNewVar_1 (stale Custom|MenuButtonClicked _x))))))
        (:then_1
          (bind _outactors (Actor|GetAllActorsOfClass "/Game/GameFolder/Player/Player_Pawn.Player_Pawn_C")))
        (:then_2
          (EventDispatchers|BindEventtoOnClicked (Variables|/Game/GameFolder/Player/PlayerHUD/Menu_HUD.Menu_HUD_C|GetButton_665 (Variables|/Game/GameFolder/Player/PlayerHUD/Main_HUD.Main_HUD_C|GetMenu_HUD_359 (Variables|Default|GetMain%20HUD))) (delegate Custom|BackButtonClicked)))
        (:then_3
          (EventDispatchers|BindEventtoOnClicked (Variables|/Game/GameFolder/Player/PlayerHUD/Main_HUD.Main_HUD_C|GetMenu (Variables|Default|GetMain%20HUD)) (delegate Custom|MenuButtonClicked)))
        (:then_4
          ;[1 1 1] Sat Deployment
          (Utilities|FlowControl|Sequence
            (:then_0
              (if (Variables|Default|GetTech%20Full)
                (if (Variables|Default|GetDone)
                  (Utilities|FlowControl|Sequence
                    (:then_0
                      (Utilities|FlowControl|Sequence
                        (:then_0
                          (bind _newtrack_4 (Timeline|Timeline_0 Play)
                            (:Update
                              (Transformation|SetRelativeLocation (Variables|Default|GetRocket) (Math|Vector|MakeVector 0.0 _newtrack_4 0.0) false false))
                            (:Finished
                              (Rendering|SetVisibility (Variables|Default|GetSat_DECIMATED) true false)
                              (Variables|Default|SetSAT_Visibility true)
                              (bind _newtrack_5 (Timeline|Timeline_2 Play)
                                (:Update
                                  (Transformation|SetWorldRotation (Variables|Default|GetRocket) (Math|Rotator|MakeRotator 0.0 0.0 _newtrack_5) false false)
                                  (bind _newtrack_4_2 (Timeline|Timeline_1 Play)
                                    (:Update
                                      (Transformation|SetRelativeLocation (Variables|Default|GetRocket) (Math|Vector|MakeVector 0.0 _newtrack_4_2 0.0) false false)
                                      (Variables|Default|SetDone false))
                                    (:Finished
                                      (Components|DestroyComponent (Variables|Default|GetRocket)))))))))
                        (:then_1
                          (Effects|SpawnEmitterAttached "/Game/GameFolder/Planet/Particles/RocketTrailParticle.RocketTrailParticle" _rocket "None" (Variables|/Script/Engine.SceneComponent|GetRelativeLocation _rocket)))))
                    (:then_1
                      (bind _newtrack_0 (Timeline|SAT%20ROT Play)
                        (:Update
                          (Transformation|SetRelativeRotation (Variables|Default|GetSat_DECIMATED) (Math|Rotator|MakeRotator 9e+01 _newtrack_0 0.0) false false))))))))
            (:then_2
              (if (== (Variables|/Game/GameFolder/Player/PlayerHUD/Main_HUD.Main_HUD_C|Gettechnology (Variables|Default|GetMain%20HUD)) 1.0)
                (Utilities|FlowControl|Delay 2.4e+02)
                (Variables|Default|SetTech%20Full true)))))))
    (:then_5
      (Utilities|FlowControl|DoOnce false
        (:Completed
          (Rendering|SetVisibility (Variables|Default|GetSat_DECIMATED) false false))))
    (:then_6
      (Utilities|FlowControl|Sequence
        (:then_0
          (if (and (Variables|/Game/GameFolder/Player/PlayerHUD/Main_HUD.Main_HUD_C|GetTooHot (Variables|Default|GetMain%20HUD)) (Variables|/Game/GameFolder/Player/PlayerHUD/Main_HUD.Main_HUD_C|GetMax%20Sun%20Toggle (Variables|Default|GetMain%20HUD)))
            (bind _newtrack_0_2 (Timeline|Onfire%20Timeline Play)
              (:Update
                (Rendering|Material|SetScalarParameterValue "/Game/GameFolder/Planet/Materials/Atmosphere.Atmosphere" "FireAtmos" _newtrack_0_2 :!class /Script/Engine.KismetMaterialLibrary)
                (Development|PrintString "")))))
        (:then_1
          (if (not (Variables|/Game/GameFolder/Player/PlayerHUD/Main_HUD.Main_HUD_C|GetMax%20Sun%20Toggle (Variables|Default|GetMain%20HUD)))
            (Timeline|Onfire%20Timeline Reverse)))))
    (:then_7
      ;[1 1 1] Set Main HUD
      (Variables|Default|SetMain%20HUD (stale EventBeginPlay _returnvalue)))))

(fn ConstructionScript)

(fn OnFireMAT
  (bind _returnvalue (Rendering|Material|CreateDynamicMaterialInstance (Variables|Default|GetAtmosphericFluid) 0 "/Game/GameFolder/Planet/Materials/OnFire_Inst.OnFire_Inst" :!class /Script/Engine.PrimitiveComponent))
  (Variables|Default|SetDynamic_MAT _returnvalue))